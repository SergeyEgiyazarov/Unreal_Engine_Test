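; BP_TurtleForward is a turtle actor that travels in a straight line toward a finish.
; Tick adds a fixed world X offset without sweep while IsStop is false, so its speed depends on frame rate.
; The Stop event, meant for reaching the finish, sets IsStop, spawns the P_Finish particle just below the turtle and stops MoveW, then destroys the actor after a short delay.
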(event `self.ReceiveTick`
  (params (DeltaSeconds :type "Float (single-precision)"))
  ;[1 1 1] Движение черепахи
  (if (not (`self.isStop`))
    (`self.K2_SetActorLocation` (+ (`self.K2_GetActorLocation`) (5.0 0.0 0.0)))))

(event `/Game/BP/BPInterface.Stop`
  ;[1 1 1] События при достижении финиша
  (set `self.isStop` true)
  (`GameplayStatics.SpawnEmitterAtLocation` "/Game/MyParticleSystem/Sprite/P_Finish.P_Finish" (+ (`self.K2_GetActorLocation`) (0.0 0.0 -20.0)))
  (`AudioComponent.Stop` (`self.MoveW`))
  (`KismetSystemLibrary.Delay` 1.0)
  (`self.K2_DestroyActor`))

(fn `UserConstructionScript`)